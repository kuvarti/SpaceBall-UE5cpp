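; Base vegetable actor that shows a collection progress bar while a Character overlaps its collision.
; Each tick during overlap, it divides the collect timer's elapsed time by CollectTime, clamps the result and feeds it to the VegetableHUD in its widget component.
; BeginPlay sets a yaw rotation value, but this graph neither applies it nor starts the timer.
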(event `self.ReceiveBeginPlay`
  (set `self.yawrotate` 1.5))

(event `self.ReceiveActorBeginOverlap`
  (params (OtherActor :type "Actor Object Reference")))

(event `self.ReceiveTick`
  (params (DeltaSeconds :type "Float (single-precision)"))
  (if (>= (`KismetArrayLibrary.Array_Length` (`PrimitiveComponent.GetOverlappingActors` (`self.collision`) "/Script/Engine.Character")) 1)
    (bind _asvegetable_hud (cast `VegetableHUD` (`WidgetComponent.GetWidget` (`self.Widget`))))
    (`VegetableHUD.setbar` _asvegetable_hud (`KismetMathLibrary.FClamp` (`KismetMathLibrary.Abs` (/ (`KismetSystemLibrary.K2_GetTimerElapsedTimeHandle` (`self.cTimerHandle`)) (`self.collectTime`)))) 1.0)))

(fn `UserConstructionScript`)